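; BP_DoorTriggerSwapper is a gameplay actor that links two collectible keys to two doors.
; On BeginPlay it binds to each key's OnCollected event, and each handler records its key as collected.
; Both handlers then call CheckAllKeysCollected, which sets AllTriggerActorsTriggered on both doors' Transporters once both keys are collected, in either order.
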(event `self.ReceiveBeginPlay`
  (add `CollectableKey.OnCollected` (`self.Key1`) (delegate `OnCollected_Key1_Event`))
  (add `CollectableKey.OnCollected` (`self.Key2`) (delegate `OnCollected_Key2_Event`)))

(event `OnCollected_Key1_Event`
  (set `self.bKey1Collected` true)
  (`self.CheckAllKeysCollected` (and (`self.bKey1Collected`) (`self.bKey2Collected`)) :!label _label))

(event `OnCollected_Key2_Event`
  (set `self.bKey2Collected` true)
  (goto _label))

(fn `CheckAllKeysCollected`
  (params (Condition :type Boolean))
  (if Condition
    (set `Transporter.AllTriggerActorsTriggered` true (`MovableActor.Transporter` (`self.Door1`)))
    (set `Transporter.AllTriggerActorsTriggered` true (`MovableActor.Transporter` (`self.Door2`)))))

(fn `UserConstructionScript`)